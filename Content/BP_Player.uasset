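; Player Blueprint that lets the player grab and release through its Grabber component.
; IA_Grab calls Grab and enters the holding state only on success, while IA_Release calls Release and exits that state.
; The holding state is an Enhanced Input mapping context, IMC_Holding, added at priority 1 on the local player subsystem and removed on release.
; Debug strings report each outcome.
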(event `self.ReceiveBeginPlay`)

(event `EnhancedInput|/Game/FirstPerson/Input/Actions/IA_Grab`
  (params (ActionValue :type Boolean) (ElapsedSeconds :type "Float (double-precision)") (TriggeredSeconds :type "Float (double-precision)") (InputAction :type "InputAction Object Reference" :default "/Game/FirstPerson/Input/Actions/IA_Grab.IA_Grab"))
  (:`Triggered`
    (bind _returnvalue (`Grabber.Grab` (`self.Grabber`)))
    (if _returnvalue
      (`self.EnterHoldingState`)
      (`KismetSystemLibrary.PrintString` "Grabbed")
      (else
        (`KismetSystemLibrary.PrintString` "Can't grab")))))

(event `EnhancedInput|/Game/FirstPerson/Input/Actions/IA_Release`
  (params (ActionValue :type Boolean) (ElapsedSeconds :type "Float (double-precision)") (TriggeredSeconds :type "Float (double-precision)") (InputAction :type "InputAction Object Reference" :default "/Game/FirstPerson/Input/Actions/IA_Release.IA_Release"))
  (:`Triggered`
    (`Grabber.Release` (`self.Grabber`))
    (`self.ExitHoldingState`)
    (`KismetSystemLibrary.PrintString` "Released")))

(fn `EnterHoldingState`
  (bind _asplayer_controller (cast `PlayerController` (`self.GetController`)))
  (message `EnhancedInputSubsystemInterface.AddMappingContext` (pcsubsystem `EnhancedInputLocalPlayerSubsystem` _asplayer_controller) "/Game/FirstPerson/Input/IMC_Holding.IMC_Holding" 1 (struct)))

(fn `ExitHoldingState`
  (bind _asplayer_controller (cast `PlayerController` (`self.GetController`)))
  (message `EnhancedInputSubsystemInterface.RemoveMappingContext` (pcsubsystem `EnhancedInputLocalPlayerSubsystem` _asplayer_controller) "/Game/FirstPerson/Input/IMC_Holding.IMC_Holding" (struct)))

(fn `UserConstructionScript`
  (`parent.UserConstructionScript`))