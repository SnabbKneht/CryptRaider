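; BP_SecretWall is a secret wall actor that unlocks while an actor tagged "Gargoyle" sits in its trigger.
; The Trigger's begin overlap sets ShouldMove to true on its ConnectedMover, and end overlap sets it back to false.
; Both events print an unlock or relock message, and the movement itself is left to the mover.
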(event `self.ReceiveBeginPlay`)

(event `self.Trigger.OnComponentBeginOverlap`
  (params (OverlappedComponent :type "PrimitiveComponent Object Reference") (OtherActor :type "Actor Object Reference") (OtherComp :type "PrimitiveComponent Object Reference") (OtherBodyIndex :type Integer) (bFromSweep :type Boolean) (SweepResult :type "HitResult Structure (by ref)"))
  (if (`self.ActorHasTag` OtherActor "Gargoyle")
    (`KismetSystemLibrary.PrintString` "Unlocking")
    (set `Mover.ShouldMove` true (`TriggerComponent.ConnectedMover` (`self.Trigger`)))))

(event `self.Trigger.OnComponentEndOverlap`
  (params (OverlappedComponent :type "PrimitiveComponent Object Reference") (OtherActor :type "Actor Object Reference") (OtherComp :type "PrimitiveComponent Object Reference") (OtherBodyIndex :type Integer))
  (if (`self.ActorHasTag` OtherActor "Gargoyle")
    (`KismetSystemLibrary.PrintString` "Relocking")
    (set `Mover.ShouldMove` false (`TriggerComponent.ConnectedMover` (`self.Trigger`)))))

(fn `UserConstructionScript`)